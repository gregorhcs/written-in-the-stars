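; Player controller for a star-connecting game that scores lines drawn on a BP_StarGrid.
; On BeginPlay it finds the star grid and adds a WB_Counter widget to the viewport.
; Releasing the left mouse button adds the grid's current line length to the star counter, updates the widget, then tells the grid to stop connecting.
; FetchCounter hands out the counter widget when it is valid.
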(event `self.ReceiveBeginPlay`
  (bind _returnvalue (`GameplayStatics.GetActorOfClass` "/Game/Blueprints/BP_StarGrid.BP_StarGrid_C"))
  (set `self.StarGrid` _returnvalue)
  (bind _returnvalue_2 (`|CreateWidget` "/Game/UI/WB_Counter.WB_Counter_C"))
  (bind _output_get (set `self.WB Counter` _returnvalue_2))
  (`UserWidget.AddToViewport` _output_get 0))

(event `Key|LeftMouseButton`
  (params (Key :type "Key Structure"))
  (:`Released`
    (`KismetSystemLibrary.PrintString` "Release")
    (bind _output_get (set `self.StarCounter` (+ (`self.StarCounter`) (`/Game/Blueprints/BP_StarGrid.CurrentLineLength` (`self.StarGrid`)))))
    (`/Game/UI/WB_Counter.Update` (`self.WB Counter`) _output_get)
    (`/Game/Blueprints/BP_StarGrid.StopConnecting` (`self.StarGrid`))))

(fn `UserConstructionScript`)