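; BP_Star is a clickable star on the star grid, storing its column and row.
; On BeginPlay it caches the player's BP_WITS_Controller, whose StarGrid receives its input.
; Clicking the star starts a connection on the grid, and moving the cursor over it adds it to that connection.
; It also exposes events to set the radius and color of its LightStar light.
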(event `self.ReceiveBeginPlay`
  (bind _asbp_wits_controller (cast `/Game/Blueprints/Core/BP_WITS_Controller` (`GameplayStatics.GetPlayerController` 0)))
  (set `self.BP WITS Controller` _asbp_wits_controller))

(event `self.ReceiveActorOnClicked`
  (params (ButtonPressed :type "Key Structure"))
  (`/Game/Blueprints/BP_StarGrid.StartConnecting` (`/Game/Blueprints/Core/BP_WITS_Controller.StarGrid` (`self.BP WITS Controller`)) self))

(event `self.ReceiveActorBeginCursorOver`
  (`/Game/Blueprints/BP_StarGrid.AddStarToConnection` (`/Game/Blueprints/Core/BP_WITS_Controller.StarGrid` (`self.BP WITS Controller`)) self))

(event `SetLightRadius`
  (params (NewRadius :type "Float (single-precision)"))
  (`LocalLightComponent.SetAttenuationRadius` (`self.Light_Star`) NewRadius))

(event `SetLightColor`
  (params (NewColor :type "LinearColor Structure"))
  (`LightComponent.SetLightColor` (`self.Light_Star`) NewColor true))

(fn `SetPosition`
  (params (Column :type Integer) (Row :type Integer))
  (set `self.Column` Column)
  (set `self.Row` Row))

(fn `UserConstructionScript`)