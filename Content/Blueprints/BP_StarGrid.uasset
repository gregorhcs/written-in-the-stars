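; Star grid manager for a constellation-style game where the player links stars on a scrolling field.
; Tick moves every BP_Star, with a timer adjusting speed periodically.
; An overlap trigger recycles rows, treating the cell array as a ring buffer and spawning replacements at the top.
; A pending BP_StarLine follows a mouse-traced indicator, locking onto connectable, unlinked neighbors, diagonals included, to chain connections.
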(event `self.ReceiveBeginPlay`
  (`|ExecutionSequence`
    (:`then_0`
      ;[0 0 0] Init Arrays
      (`KismetArrayLibrary.Array_Resize` (`self.Grid Crosses`) (* (+ (`self.Columns`) 1) (+ (`self.Rows`) 1)))
      (`KismetArrayLibrary.Array_Resize` (`self.GridCells`) (* (`self.Columns`) (`self.Rows`)))
      (set `self.TopRow` (- (`self.Rows`) 1)))
    (:`then_1`
      ;[0 0 0] Draw Test Field
      (for _index (range (`self.Columns`))
        (for _index_2 (range (`self.Rows`))
          (`self.SpawnGridCellInit` _index _index_2))))
    (:`then_2`
      ;[0 0 0] Fetch Mouse Indicator Actor
      (bind _outactors (`GameplayStatics.GetAllActorsWithTag` "MouseIndicatorActor"))
      (set `self.MouseIndicatorActor` (`|GetArrayItem` _outactors)))
    (:`then_3`
      ;[0 0 0] Speed Increases
      (`KismetSystemLibrary.K2_SetTimerDelegate` (delegate `IncreaseSpeed`) 10.0 true))))

(event `IncreaseSpeed`
  ;[0 0 0] Speed Increases
  (set `self.MoveSpeed` (+ (`self.MoveSpeed`) -0.01)))

(event `self.Collision_RowStreaming.OnComponentBeginOverlap`
  (params (OverlappedComponent :type "PrimitiveComponent Object Reference") (OtherActor :type "Actor Object Reference") (OtherComp :type "PrimitiveComponent Object Reference") (OtherBodyIndex :type Integer) (bFromSweep :type Boolean) (SweepResult :type "HitResult Structure (by ref)"))
  ;[0 0 0] Streaming
  (`|ExecutionSequence`
    (:`then_0`
      (if (`KismetMathLibrary.ClassIsChildOf` (`GameplayStatics.GetObjectClass` OtherActor) "/Game/Blueprints/BP_Star.BP_Star_C")
        (set `self.TopRow` (mod (+ (`self.TopRow`) 1) (`self.Rows`)))
        (for _index (range (`self.Columns`))
          (`self.K2_DestroyActor` (`|GetArrayItem` (`self.GridCells`) (`self.GetGridCellArrayIndex` _index (`self.TopRow`))))
          (`self.SpawnGridCellTop` (`self.TopRow`) _index))))
    (:`then_1`
      (if (`KismetMathLibrary.ClassIsChildOf` (`GameplayStatics.GetObjectClass` OtherActor) "/Script/Niagara.NiagaraActor")
        (`self.K2_DestroyActor` OtherActor)))))

(event `self.ReceiveTick`
  (params (DeltaSeconds :type "Float (single-precision)"))
  ;[0 0 0] Movement
  (`self.UpdateConnecting`)
  (`|ExecutionSequence`
    (:`then_0`
      (for _array_element (`self.GridCells`)
        (`self.K2_AddActorLocalOffset` _array_element (`KismetMathLibrary.MakeVector` (`self.MoveSpeed`)) true false)))))

(fn `AddStarToConnection`
  (params (StarHovered :type "/Game/Blueprints/BP_Star Object Reference"))
  (returns (`Connected?` :type Boolean))
  (bind _starhovered (`local.StarHovered`))
  (bind _starhovered_2 (`local.StarHovered`))
  (bind _starstart (`self.StarStart`))
  (bind _currentconnectingstarline (`self.CurrentConnectingStarLine`))
  (bind _starstart_2 (`self.StarStart`))
  (`/Engine/EditorBlueprintResources/StandardMacros.IsValid` (`self.StarStart`)
    (:`Is Valid`
      (`/Engine/EditorBlueprintResources/StandardMacros.IsValid` (`self.CurrentConnectingStarLine`)
        (:`Is Valid`
          (if (and (`/Game/Blueprints/BP_Star.CanBeConnected?` _starhovered) (`/Game/Blueprints/BP_Star.CanBeConnected?` _starstart) (!= _starhovered _starstart) (not (`self.StarsConnected?` _starhovered _starstart)) (`self.StarsAdjacent?` _starhovered _starstart))
            (set `/Game/Blueprints/BP_StarLine.ActorEnd` (`local.StarHovered`) _currentconnectingstarline)
            (`/Game/Blueprints/BP_StarLine.UpdatePosition` _currentconnectingstarline)
            (`/Game/Blueprints/BP_Star.ConnectTo` (`self.StarStart`) (`local.StarHovered`) false)
            (`/Game/Blueprints/BP_Star.ConnectTo` (`local.StarHovered`) (`self.StarStart`) true)
            (`/Engine/EditorBlueprintResources/StandardMacros.IncrementInt` (`self.CurrentLineLength`)
              (:`  `
                (`KismetSystemLibrary.PrintText` (`|FormatText` "Connect: {A}/{B} and {X}/{Y}" (`/Game/Blueprints/BP_Star.Column` _starstart_2) (`/Game/Blueprints/BP_Star.Row` _starstart_2) (`/Game/Blueprints/BP_Star.Column` _starhovered_2) (`/Game/Blueprints/BP_Star.Row` _starhovered_2)))
                (set `self.StarStart` (`local.StarHovered`))
                (set `self.CurrentConnectingStarLine` null)
                (return true)))
            (else
              _)))
        (:`Is Not Valid`
          _)))
    (:`Is Not Valid`
      _))
  (return false))

(fn `DrawStarLine`
  (params (ActorStart :type "Actor Object Reference") (ActorEnd :type "Actor Object Reference"))
  (returns (`Star Line` :type "/Game/Blueprints/BP_StarLine Object Reference"))
  (bind _returnvalue (`|SpawnActorFromClass` "/Game/Blueprints/BP_StarLine.BP_StarLine_C" (`KismetMathLibrary.Conv_VectorToTransform` (`self.K2_GetActorLocation` ActorStart)) "Undefined" "OverrideRootScale" null null))
  (`KismetArrayLibrary.Array_Add` (`self.StarLines`) _returnvalue)
  (set `/Game/Blueprints/BP_StarLine.ActorStart` ActorStart _returnvalue)
  (set `/Game/Blueprints/BP_StarLine.ActorEnd` ActorEnd _returnvalue)
  (`/Game/Blueprints/BP_StarLine.UpdatePosition` _returnvalue)
  (return _returnvalue))

(fn `StartConnecting`
  (params (StarStart :type "/Game/Blueprints/BP_Star Object Reference"))
  (set `self.StarStart` StarStart)
  (set `self.CurrentLineLength` 0))

(fn `StopConnecting`
  (bind _currentconnectingstarline (`self.CurrentConnectingStarLine`))
  (`/Engine/EditorBlueprintResources/StandardMacros.IsValid` (`self.StarStart`)
    (:`Is Valid`
      (set `self.StarStart` null)
      (`KismetArrayLibrary.Array_RemoveItem` (`self.StarLines`) _currentconnectingstarline)
      (`self.K2_DestroyActor` _currentconnectingstarline)
      (set `self.CurrentLineLength` 0))))

(fn `UpdateConnecting`
  (`/Engine/EditorBlueprintResources/StandardMacros.IsValid` (`self.StarStart`)
    (:`Is Valid`
      (`self.UpdateMouseWorldPosition`)
      (`/Engine/EditorBlueprintResources/StandardMacros.IsValid` (`self.CurrentConnectingStarLine`)
        (:`Is Not Valid`
          (bind _star_line (`self.DrawStarLine` (`self.StarStart`) (`self.MouseIndicatorActor`)))
          (set `self.CurrentConnectingStarLine` _star_line))))))

(fn `UpdateMouseWorldPosition`
  (returns (ReturnValue :type "Vector Structure"))
  (bind _returnvalue (`WidgetLayoutLibrary.GetViewportScale`))
  (bind _returnvalue_2 (`WidgetLayoutLibrary.GetMousePositionOnViewport`))
  (bind (_x _y) (`KismetMathLibrary.BreakVector2D` _returnvalue_2))
  (bind (_worldposition _worlddirection) (`GameplayStatics.DeprojectScreenToWorld` (`GameplayStatics.GetPlayerController` 0) (`KismetMathLibrary.MakeVector2D` (* _x _returnvalue) (* _y _returnvalue))))
  (bind _outhit (`KismetSystemLibrary.LineTraceSingle` _worldposition (+ _worldposition (* _worlddirection 2000.0)) "TraceTypeQuery1"))
  (bind _returnvalue_3 (`KismetMathLibrary.MakeVector` (.x (`self.K2_GetActorLocation` (`self.MouseIndicatorActor`))) (.y (`.Location` (`GameplayStatics.BreakHitResult` _outhit))) (.z (`.Location` (`GameplayStatics.BreakHitResult` _outhit)))))
  (`self.K2_SetActorLocation` (`self.MouseIndicatorActor`) _returnvalue_3 false false)
  (return _returnvalue_3))

(fn `UserConstructionScript`)