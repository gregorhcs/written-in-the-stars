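; BP_StarLine is an actor that keeps a Niagara effect spanning two referenced actors, apparently as a line between stars.
; Every Tick, UpdatePosition moves the actor to ActorStart's location with a swept move.
; It then passes ActorEnd's location to the Niagara component's EndPosition variable, with each reference checked for validity first.
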(event `self.ReceiveTick`
  (params (DeltaSeconds :type "Float (single-precision)"))
  (`self.UpdatePosition`))

(fn `UpdatePosition`
  (`|ExecutionSequence`
    (:`then_0`
      (`/Engine/EditorBlueprintResources/StandardMacros.IsValid` (`self.ActorStart`)
        (:`Is Valid`
          (`self.K2_SetActorLocation` (`self.K2_GetActorLocation` (`self.ActorStart`)) true))))
    (:`then_1`
      (`/Engine/EditorBlueprintResources/StandardMacros.IsValid` (`self.ActorEnd`)
        (:`Is Valid`
          (`NiagaraComponent.SetVariableVec3` (`self.Niagara`) "EndPosition" (`self.K2_GetActorLocation` (`self.ActorEnd`))))))))

(fn `UserConstructionScript`)